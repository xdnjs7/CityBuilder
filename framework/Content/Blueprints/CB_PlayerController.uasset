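; Player controller that drives a movable camera pawn and handles mouse-based placement of a building, likely for a builder-style game.
; Input events cast the controlled pawn to CB_MovingCameraC and forward movement, rotation, pitch and zoom, with mouse orbit and pitch active only while right-click is held.
; BeginPlay selects a sample building and spawns it at the cursor, Tick updates its position to the mouse, and left-click calls OnLeftMouseClick.
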(event `InputAxis|Rotate`
  (params (AxisValue :type "Float (single-precision)"))
  (bind _ascb_moving_camera_c (cast `/Game/Blueprints/CB_MovingCameraC` (`self.K2_GetPawn`)))
  (`CB_MovingCamera.CameraOrbit` _ascb_moving_camera_c AxisValue))

(event `InputAxis|MoveForward`
  (params (AxisValue :type "Float (single-precision)"))
  (bind _ascb_moving_camera_c (cast `/Game/Blueprints/CB_MovingCameraC` (`self.K2_GetPawn`)))
  (`CB_MovingCamera.MoveForward` _ascb_moving_camera_c AxisValue))

(event `InputAxis|MoveRight`
  (params (AxisValue :type "Float (single-precision)"))
  (bind _ascb_moving_camera_c (cast `/Game/Blueprints/CB_MovingCameraC` (`self.K2_GetPawn`)))
  (`CB_MovingCamera.MoveRight` _ascb_moving_camera_c AxisValue))

(event `InputAction|ZoomIn`
  (params (Key :type "Key Structure"))
  (:`Pressed`
    (bind _ascb_moving_camera_c (cast `/Game/Blueprints/CB_MovingCameraC` (`self.K2_GetPawn`)))
    (`CB_MovingCamera.CameraZoom` _ascb_moving_camera_c -1.0)))

(event `InputAction|ZoomOut`
  (params (Key :type "Key Structure"))
  (:`Pressed`
    (bind _ascb_moving_camera_c (cast `/Game/Blueprints/CB_MovingCameraC` (`self.K2_GetPawn`)))
    (`CB_MovingCamera.CameraZoom` _ascb_moving_camera_c 1.0)))

(event `InputAxis|CameraPitch`
  (params (AxisValue :type "Float (single-precision)"))
  (bind _ascb_moving_camera_c (cast `/Game/Blueprints/CB_MovingCameraC` (`self.K2_GetPawn`)))
  (`CB_MovingCamera.CameraPitch` _ascb_moving_camera_c AxisValue))

(event `InputAction|MouseRightClick`
  (params (Key :type "Key Structure"))
  (:`Pressed`
    (set `self.RightButtonPressed` true))
  (:`Released`
    (set `self.RightButtonPressed` false)))

(event `InputAxis|MouseX`
  (params (AxisValue :type "Float (single-precision)"))
  (if (`self.RightButtonPressed`)
    (bind _ascb_moving_camera_c (cast `/Game/Blueprints/CB_MovingCameraC` (`self.K2_GetPawn`)))
    (`CB_MovingCamera.CameraOrbit` _ascb_moving_camera_c AxisValue)))

(event `InputAxis|MouseY`
  (params (AxisValue :type "Float (single-precision)"))
  (if (`self.RightButtonPressed`)
    (bind _ascb_moving_camera_c (cast `/Game/Blueprints/CB_MovingCameraC` (`self.K2_GetPawn`)))
    (`CB_MovingCamera.CameraPitch` _ascb_moving_camera_c AxisValue)))

(event `self.ReceiveBeginPlay`
  (set `self.buildingType` "/Game/Blueprints/SampleBuilding.SampleBuilding_C")
  (`self.SpawnActorAtMousePosition`)
  (`self.SetupInputComponent`))

(event `self.ReceiveTick`
  (params (DeltaSeconds :type "Float (single-precision)"))
  (`self.UpdateActorPositionToMousePosition`))

(event `Key|LeftMouseButton`
  (params (Key :type "Key Structure"))
  (:`Pressed`
    (`self.OnLeftMouseClick`)))

(fn `UserConstructionScript`)