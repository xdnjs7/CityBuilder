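; CB_CameraController is a camera controller Blueprint with a CharacterMovement component that ties its movement speed to the zoom level of its spring arm.
; On BeginPlay it caches the initial max walk speed, then calls UpdateMovementSpeed.
; That function scales the cached speed by the ratio of MCSpringArm's arm length to the minimum zoom, so a longer arm gives proportionally faster movement.
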(event `self.ReceiveBeginPlay`
  (set `self.InitialMovementSpeed` (`CharacterMovementComponent.MaxWalkSpeed` (`self.CharacterMovement`)))
  (`self.UpdateMovementSpeed`))

(fn `UpdateMovementSpeed`
  (set `CharacterMovementComponent.MaxWalkSpeed` (* (`self.InitialMovementSpeed`) (/ (`SpringArmComponent.TargetArmLength` (`self.MCSpringArm`)) (`self.ZoomMin`))) (`self.CharacterMovement`)))

(fn `UserConstructionScript`)