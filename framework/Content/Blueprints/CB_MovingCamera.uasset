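; CB_MovingCamera is a Character-based player camera that moves, orbits, pitches and zooms from axis input.
; Movement follows control yaw only, and orbit adds controller yaw input.
; Pitch sets the spring arm's world rotation through CameraPitchCal, while zoom changes its arm length within clamped limits.
; It stores the initial walk speed on BeginPlay and calls UpdateMovementSpeed then and on every zoom input.
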(event `self.ReceiveBeginPlay`
  (set `self.InitialMovementSpeed` (`CharacterMovementComponent.MaxWalkSpeed` (`self.CharacterMovement`)))
  (`self.UpdateMovementSpeed`))

(event `self.CameraOrbit`
  (params (Value :type "Float (single-precision)"))
  (`self.AddControllerYawInput` (* Value (`self.OrbitSpeed`))))

(event `self.CameraPitch`
  (params (Value :type "Float (single-precision)"))
  (bind _returnvalue (`self.CameraPitchCal` Value))
  (`SceneComponent.K2_SetWorldRotation` (`self.SpringArm`) _returnvalue false false))

(event `self.MoveForward`
  (params (Value :type "Float (single-precision)"))
  (`self.AddMovementInput` (`KismetMathLibrary.GetForwardVector` (`KismetMathLibrary.MakeRotator` 0.0 0.0 (.yaw (`self.GetControlRotation`)))) Value))

(event `self.MoveRight`
  (params (Value :type "Float (single-precision)"))
  (`self.AddMovementInput` (`KismetMathLibrary.GetRightVector` (`KismetMathLibrary.MakeRotator` 0.0 0.0 (.yaw (`self.GetControlRotation`)))) Value))

(event `self.CameraZoom`
  (params (Value :type "Float (single-precision)"))
  (bind _springarm (`self.SpringArm`))
  (set `SpringArmComponent.TargetArmLength` (`KismetMathLibrary.FClamp` (+ (* Value (`self.ZoomSpeed`)) (`SpringArmComponent.TargetArmLength` _springarm)) (`self.ZoomMin`) (`self.ZoomMax`)) _springarm)
  (`self.UpdateMovementSpeed`))

(fn `UserConstructionScript`)